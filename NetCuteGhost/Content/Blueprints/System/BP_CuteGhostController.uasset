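; Player controller for the Cute Ghost pawn, moving it along world X and Y.
; On BeginPlay, after a short delay, it adopts its ghost and views a WorldCamera-tagged actor, or spawns and possesses a new ghost, then passes it the controller ID.
; Axis inputs offset the ghost directly without sweep; with UseConsoleForControl set, Tick moves it from stored axis values and per-axis flags instead.
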(event `self.ReceiveBeginPlay`
  (`KismetSystemLibrary.Delay` 0.5)
  (bind _asbp_cute_ghost (cast `/Game/Characters/BP_CuteGhost` (`self.K2_GetPawn`))
    (:`then`
      (set `self.ControlledGhost` _asbp_cute_ghost)
      (bind _outactors (`GameplayStatics.GetAllActorsWithTag` "WorldCamera"))
      (`self.SetViewTargetWithBlend` (`|GetArrayItem` _outactors)))
    (:`CastFailed`
      (bind _returnvalue (`|SpawnActorFromClass` "/Game/Characters/BP_CuteGhost.BP_CuteGhost_C" (`KismetMathLibrary.MakeTransform` (0.0 0.0 0.0)) "AdjustIfPossibleButAlwaysSpawn" "OverrideRootScale" null null))
      (bind _output_get (set `self.ControlledGhost` _returnvalue))
      (`self.Possess` _output_get)))
  (bind _returnvalue_2 (`GameplayStatics.GetPlayerControllerID` self))
  (set `/Game/Characters/BP_CuteGhost.ControllerID` _returnvalue_2 (`self.ControlledGhost`)))

(event `self.ReceiveTick`
  (params (DeltaSeconds :type "Float (single-precision)"))
  (bind _axisvalue (`self.AxisValue`))
  (bind _axisscale (`self.AxisScale`))
  (if (`self.bUseConsoleForControl`)
    (`|ExecutionSequence`
      (:`then_0`
        (if (`self.bCanMoveXAxis`)
          (`self.MoveXAxis` _axisvalue _axisscale)))
      (:`then_1`
        (if (`self.bCanMoveYAxis`)
          (`self.MoveYAxis` _axisvalue _axisscale))))))

(event `InputAxis|XAxis`
  (params (AxisValue :type "Float (single-precision)"))
  (if (not (`self.bUseConsoleForControl`))
    (`self.MoveXAxis` AxisValue)))

(event `InputAxis|YAxis`
  (params (AxisValue :type "Float (single-precision)"))
  (if (not (`self.bUseConsoleForControl`))
    (`self.MoveYAxis` AxisValue)))

(fn `MoveXAxis`
  (params (Value :type "Float (double-precision)" :default 0.0) (Scale :type "Float (double-precision)" :default 1.0))
  (bind _controlledghost (`self.ControlledGhost`))
  (if (`KismetSystemLibrary.IsValid` _controlledghost)
    (`self.K2_AddActorWorldOffset` _controlledghost (* (5.0 0.0 0.0) (* Value Scale)) false false)))

(fn `MoveYAxis`
  (params (Value :type "Float (double-precision)") (Scale :type "Float (double-precision)" :default 1.0))
  (bind _controlledghost (`self.ControlledGhost`))
  (if (`KismetSystemLibrary.IsValid` _controlledghost)
    (`self.K2_AddActorWorldOffset` _controlledghost (* (0.0 5.0 0.0) (* Value Scale)) false false)))

(fn `UserConstructionScript`)