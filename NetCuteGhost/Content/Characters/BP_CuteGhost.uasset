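; Ghost character that tints its emissive mesh material with one of eight color pairs chosen by ControllerID.
; One second after BeginPlay it creates a dynamic material instance, retrying each second while ControllerID is -1.
; SetDynamicMaterialByID then sets the LowColor and HighColor parameters.
; That call does not wait for the retry loop, so a late ID creates the material without coloring it here.
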(event `self.ReceiveBeginPlay`
  (`KismetSystemLibrary.Delay` 1.0)
  (`|ExecutionSequence`
    (:`then_0`
      (if (`KismetSystemLibrary.IsValid` (`self.GetController`))
        _))
    (:`then_1`
      (if (!= (`self.ControllerID`) -1) :!label _label
        (bind _returnvalue (`PrimitiveComponent.CreateDynamicMaterialInstance` (`self.StaticMesh`) 0 "/Game/Characters/MI_GhostEmissive_inst.MI_GhostEmissive_inst" "None"))
        (if (`KismetSystemLibrary.IsValid` _returnvalue)
          (set `self.GhostDynMat` _returnvalue))
        (else
          (`KismetSystemLibrary.Delay` 1.0)
          (goto _label))))
    (:`then_2`
      (`self.SetDynamicMaterialByID`))))

(fn `SetDynamicMaterialByID`
  (bind _controllerid (`self.ControllerID`))
  (bind _ghostdynmat (`self.GhostDynMat`))
  (if (!= (`self.ControllerID`) -1)
    (if (`KismetSystemLibrary.IsValid` (`self.GhostDynMat`))
      (`|ExecutionSequence`
        (:`then_0`
          (if (== _controllerid 0)
            (`MaterialInstanceDynamic.SetVectorParameterValue` _ghostdynmat "LowColor" (struct :`R` 2.0 :`A` 1.0))
            (`MaterialInstanceDynamic.SetVectorParameterValue` _ghostdynmat "HighColor" (struct :`R` 10.0 :`A` 1.0))))
        (:`then_1`
          (if (== _controllerid 1)
            (`MaterialInstanceDynamic.SetVectorParameterValue` _ghostdynmat "LowColor" (struct :`R` 2.0 :`G` 1.0 :`A` 1.0))
            (`MaterialInstanceDynamic.SetVectorParameterValue` _ghostdynmat "HighColor" (struct :`R` 10.0 :`G` 5.0 :`A` 1.0))))
        (:`then_2`
          (if (== _controllerid 2)
            (`MaterialInstanceDynamic.SetVectorParameterValue` _ghostdynmat "LowColor" (struct :`R` 2.0 :`G` 1.75 :`A` 1.0))
            (`MaterialInstanceDynamic.SetVectorParameterValue` _ghostdynmat "HighColor" (struct :`R` 10.0 :`G` 8.75 :`A` 1.0))))
        (:`then_3`
          (if (== _controllerid 3)
            (`MaterialInstanceDynamic.SetVectorParameterValue` _ghostdynmat "LowColor" (struct :`G` 2.0 :`B` 0.4 :`A` 1.0))
            (`MaterialInstanceDynamic.SetVectorParameterValue` _ghostdynmat "HighColor" (struct :`G` 10.0 :`B` 2.0 :`A` 1.0))))
        (:`then_4`
          (if (== _controllerid 4)
            (`MaterialInstanceDynamic.SetVectorParameterValue` _ghostdynmat "LowColor" (struct :`G` 0.4 :`B` 2.0 :`A` 1.0))
            (`MaterialInstanceDynamic.SetVectorParameterValue` _ghostdynmat "HighColor" (struct :`G` 2.0 :`B` 10.0 :`A` 1.0))))
        (:`then_5`
          (if (== _controllerid 5)
            (`MaterialInstanceDynamic.SetVectorParameterValue` _ghostdynmat "LowColor" (struct :`B` 2.0 :`A` 1.0))
            (`MaterialInstanceDynamic.SetVectorParameterValue` _ghostdynmat "HighColor" (struct :`B` 10.0 :`A` 1.0))))
        (:`then_6`
          (if (== _controllerid 6)
            (`MaterialInstanceDynamic.SetVectorParameterValue` _ghostdynmat "LowColor" (struct :`R` 1.0 :`B` 2.0 :`A` 1.0))
            (`MaterialInstanceDynamic.SetVectorParameterValue` _ghostdynmat "HighColor" (struct :`R` 5.0 :`B` 10.0 :`A` 1.0))))
        (:`then_7`
          (if (== _controllerid 7)
            (`MaterialInstanceDynamic.SetVectorParameterValue` _ghostdynmat "LowColor" (struct :`R` 2.0 :`G` 0.001031 :`B` 1.4 :`A` 1.0))
            (`MaterialInstanceDynamic.SetVectorParameterValue` _ghostdynmat "HighColor" (struct :`R` 10.0 :`B` 7.0 :`A` 1.0))))))))

(fn `UserConstructionScript`)